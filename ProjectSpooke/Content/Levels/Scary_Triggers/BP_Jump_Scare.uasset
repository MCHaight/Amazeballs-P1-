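; BP_Jump_Scare is a one-shot jump scare trigger that flashes a scare screen and hurts the player.
; When BP_FP_Character first overlaps the trigger box, a DoOnce creates WAC_Scare_Widget, adds it to the viewport and applies light damage to the character.
; It also starts a short non-looping timer, apparently meant to fire RemoveWiget, which takes the widget off screen.
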(event OnComponentBeginOverlap(Trigerbox)
  (params (OverlappedComponent :type Primitive%20Component%20Object%20Reference) (OtherActor :type Actor%20Object%20Reference) (OtherComp :type Primitive%20Component%20Object%20Reference) (OtherBodyIndex :type Integer) (bFromSweep :type Boolean) (SweepResult :type Hit%20Result%20Structure%20%28by%20ref%29))
  (bind _asbp_fp_character (Utilities|Casting|CastToBP_FP_Character OtherActor))
  (Utilities|FlowControl|DoOnce false
    (:Completed
      (Variables|Default|SetAs%20BP%20FP%20Character _asbp_fp_character)
      (bind _returnvalue (UserInterface|CreateWidget "/Game/Levels/Scary_Triggers/WAC_Scare_Widget.WAC_Scare_Widget_C" (Game|GetPlayerController 0)))
      (Variables|Default|SetScare%20screen _returnvalue)
      (UserInterface|Viewport|AddtoViewport _returnvalue 0)
      (Utilities|Time|SetTimerbyEvent (EventDispatchers|CreateEvent :!event Custom|Remove%20Wiget) 0.4)
      (Game|Damage|ApplyDamage (Variables|Default|GetAs%20BP%20FP%20Character) 1e+01 0 0))))

(event Custom|Remove%20Wiget
  (Widget|RemovefromParent (Variables|Default|GetScare%20screen)))

(event EventBeginPlay)

(event Collision|EventActorBeginOverlap
  (params (OtherActor :type Actor%20Object%20Reference)))

(event EventTick
  (params (DeltaSeconds :type Float%20%28single-precision%29)))

(fn ConstructionScript)