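; BP_Dodge_Ball is a throwable dodge ball pickup, built on a parent pickup Blueprint.
; PickUp turns off physics on the static mesh before running the parent pickup logic.
; UseFunction detaches the mesh in world space, restores collision and physics, then launches it along the player camera's forward vector with a large, mass-independent AddForce.
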(event EventBeginPlay
  (|CallParentFunction) ; This node is disabled and will not be called.\nDrag off pins to build functionality.
)

(event Collision|EventActorBeginOverlap
  (params (OtherActor :type Actor%20Object%20Reference)))

(event EventTick
  (params (DeltaSeconds :type Float%20%28single-precision%29)))

(event EventPickUp
  (Physics|SetSimulatePhysics (Variables|Default|GetStaticMesh) false)
  (|CallParentFunction))

(event EventUseFunction
  (bind _staticmesh (Variables|Default|GetStaticMesh))
  (bind _staticmesh_2 (Variables|Default|GetStaticMesh))
  (Transformation|DetachFromComponent (Variables|Default|GetStaticMesh) "KeepWorld" "KeepWorld" "KeepRelative" true)
  (Collision|SetCollisionEnabled _staticmesh "QueryAndPhysics")
  (Physics|SetSimulatePhysics _staticmesh_2 true)
  (Physics|AddForce _staticmesh (* (Math|Vector|GetForwardVector (Variables|/Game/PlayerCharacter/Player_Systems/BP_FP_Character.BP_FP_Character_C|GetCamera (Variables|Default|GetPlayer))) "200000.000000,200000.000000,200000.000000") (Transformation|GetAttachSocketName _staticmesh_2) true))

(fn ConstructionScript
  (|CallParentFunction))