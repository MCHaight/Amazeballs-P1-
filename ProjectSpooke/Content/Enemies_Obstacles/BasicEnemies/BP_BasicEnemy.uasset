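; BP_BasicEnemy is a basic AI enemy whose Blueprint handles the search behavior after it reaches a target's last known location.
; LookAround uses two chained timelines to sweep the root's yaw 90 degrees left, then across to the right, pausing after each turn.
; It then clears the blackboard's last-location key, flags that patrol needs resetting and sets its RectLight to pale yellow.
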(event Custom|LookAround
  ;[1 1 1] Look around after reaching targets last known location
  (Variables|Default|SetLookAroundRotation (Transformation|GetWorldRotation (Variables|Transformation|GetRootComponent)))
  (bind _newtrack_0 (Timeline|LookLeft Play)
    (:Update
      (Transformation|SetWorldRotation (Variables|Transformation|GetRootComponent) (Math|Rotator|MakeRotator (.roll (Variables|Default|GetLookAroundRotation)) (.pitch (Variables|Default|GetLookAroundRotation)) (Math|Float|Lerp (.yaw (Variables|Default|GetLookAroundRotation)) (- (.yaw (Variables|Default|GetLookAroundRotation)) 9e+01) _newtrack_0)) true false))
    (:Finished
      (Utilities|FlowControl|Delay 0.45)
      (bind _newtrack_0_2 (Timeline|LookRight Play)
        (:Update
          (Transformation|SetWorldRotation (Variables|Transformation|GetRootComponent) (Math|Rotator|MakeRotator (.roll (Variables|Default|GetLookAroundRotation)) (.pitch (Variables|Default|GetLookAroundRotation)) (Math|Float|Lerp (- (.yaw (Variables|Default|GetLookAroundRotation)) 9e+01) (+ (.yaw (Variables|Default|GetLookAroundRotation)) 9e+01) _newtrack_0_2)) true false))
        (:Finished
          (Utilities|FlowControl|Delay 0.45)
          (AI|Components|Blackboard|ClearValue (AI|GetBlackboard 0) (Utilities|Name|MakeLiteralName "TargetLastLocation"))
          (AI|Components|Blackboard|SetValueasBool (AI|GetBlackboard 0) (Utilities|Name|MakeLiteralName "ResetPatrolNeeded") true)
          (Rendering|Components|Light|SetLightColor (Variables|Default|GetRectLight) "(R=0.964686,G=1.000000,B=0.637597,A=1.000000)" false))))))

(event EventBeginPlay)

(fn ConstructionScript)