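; AI controller for basic enemies that runs a behavior tree on possess and feeds it player perception.
; Perception updates for the player pawn, unless it is the ghost player, store successful stimulus locations in the TargetLastLocation blackboard key.
; ChaseTarget is set only while the player is perceived by sight and cleared otherwise, so other senses yield just a location.
; These updates also refresh the controlled BP_BasicEnemy's aggro light color.
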(event OnTargetPerceptionUpdated(AIPerception)
  (params (Actor :type Actor%20Object%20Reference) (Stimulus :type AI%20Stimulus%20Structure))
  (bind (_stimuluslocation _bsuccessfullysensed) (Utilities|Struct|BreakAIStimulus Stimulus))
  (bind _returnvalue (Game|Player|GetPlayerPawn 0))
  ;[1 1 1] Target (Player) perception and corresponding blackboard value setting
  (if (and (== Actor _returnvalue) (not (.bSuccess (Utilities|Casting|CastToBP_Ghost_Player _returnvalue))))
    (if _bsuccessfullysensed
      (AI|Components|Blackboard|SetValueasVector (AI|GetBlackboard 0) (Utilities|Name|MakeLiteralName "TargetLastLocation") _stimuluslocation)
      (if (not (== (Utilities|Array|FindItem (Class|AIPerceptionComponent|GetCurrentlyPerceivedActors (Variables|Controller|GetAIPerception) "/Script/AIModule.AISense_Sight") (Game|Player|GetPlayerPawn 0)) -1))
        (AI|Components|Blackboard|SetValueasObject (AI|GetBlackboard 0) (Utilities|Name|MakeLiteralName "ChaseTarget") Actor)
        (else
          (AI|Components|Blackboard|SetValueasObject (AI|GetBlackboard 0) (Utilities|Name|MakeLiteralName "ChaseTarget") 0 :!label _label)))
      (else
        (goto _label)))
    (bind _asbp_basic_enemy (Utilities|Casting|CastToBP_BasicEnemy (Pawn|GetControlledPawn)))
    (Default|SetAggroLightcolor _asbp_basic_enemy)))

(event EventPossess
  (params (PossessedPawn :type Pawn%20Object%20Reference))
  (AI|RunBehaviorTree (Variables|Default|GetBehaviorTreeToRun)))

(fn ConstructionScript)