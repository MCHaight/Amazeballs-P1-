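; Blind nurse enemy Blueprint, a special enemy that works with an AI Blackboard and signals its aggro state through a rect light.
; Its LookAround event clears the last known target location and marks patrol points as unset in the Blackboard.
; The same event switches the light back to its no-aggro color.
; BeginPlay, Tick and overlap events are disabled, and the construction script only calls the parent.
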(event EventBeginPlay
  (|CallParentFunction) ; This node is disabled and will not be called.\nDrag off pins to build functionality.
)

(event Collision|EventActorBeginOverlap
  (params (OtherActor :type Actor%20Object%20Reference)))

(event EventTick
  (params (DeltaSeconds :type Float%20%28single-precision%29)))

(event EventLookAround
  (AI|Components|Blackboard|ClearValue (AI|GetBlackboard 0) (Utilities|Name|MakeLiteralName "TargetLastLocation"))
  (AI|Components|Blackboard|SetValueasBool (AI|GetBlackboard 0) (Utilities|Name|MakeLiteralName "PatrolPointsSet") false)
  (Rendering|Components|Light|SetLightColor (Variables|Default|GetRectLight) (Variables|Default|GetNo%20Aggro%20Color) false))

(fn ConstructionScript
  (|CallParentFunction))